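; Test actor that paints a fading trail where the player pawn moves over a reference plane.
; Tick converts the pawn's position to plane-relative UVs and stamps through an accumulation material once it moves far enough.
; A looping timer runs decay passes through that material, with the factor derived from a half-life.
; Both passes ping-pong between two render targets and pass the latest to the plane's RVT writer material.
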(event Custom|DecayTick
  (bind _mid (Variables|Default|GetMID))
  (bind _mid_2 (Variables|Default|GetMID))
  (bind _mid_path (Variables|Default|GetMID_Path))
  (bind _mid_3 (Variables|Default|GetMID))
  (Rendering|Material|SetScalarParameterValue _mid_3 "StampStrength" 0.0 :!class /Script/Engine.MaterialInstanceDynamic)
  (Rendering|Material|SetScalarParameterValue _mid_3 "Decay" (Variables|Default|GetDecay) :!class /Script/Engine.MaterialInstanceDynamic)
  (if (Variables|Default|GetUseA_Decay)
    (Rendering|Material|SetTextureParameterValue _mid "CurrentRT" "/Game/Materials/RT_Test_A.RT_Test_A")
    (Rendering|DrawMaterialtoRenderTarget "/Game/Materials/RT_Test_B.RT_Test_B" _mid_2)
    (Rendering|Material|SetTextureParameterValue _mid_path "CurrentRT" "/Game/Materials/RT_Test_B.RT_Test_B")
    (else
      (Rendering|Material|SetTextureParameterValue _mid "CurrentRT" "/Game/Materials/RT_Test_B.RT_Test_B")
      (Rendering|DrawMaterialtoRenderTarget "/Game/Materials/RT_Test_A.RT_Test_A" _mid_2)
      (Rendering|Material|SetTextureParameterValue _mid_path "CurrentRT" "/Game/Materials/RT_Test_A.RT_Test_A")))
  (Variables|Default|SetUseA_Decay (not (Variables|Default|GetUseA_Decay))))

(event EventBeginPlay
  (CallFunction|ReferencePlanesTransform (Variables|Default|GetPlaneRef))
  (CallFunction|ClearAllRTs)
  (bind _returnvalue (Rendering|Material|CreateDynamicMaterialInstance "/Game/Materials/M_Accumulate.M_Accumulate" "None" "None" :!class /Script/Engine.KismetMaterialLibrary))
  (Variables|Default|SetMID _returnvalue)
  (bind _returnvalue_2 (Rendering|Material|CreateDynamicMaterialInstance (Variables|/Script/Engine.StaticMeshActor|GetStaticMeshComponent (Variables|Default|GetPlaneRef)) 0 "/Game/Materials/RTRVT/M_RVTWriter.M_RVTWriter" "None" :!class /Script/Engine.PrimitiveComponent))
  (bind _output_get (Variables|Default|SetMID_Path _returnvalue_2))
  (Rendering|Material|SetTextureParameterValue _output_get "CurrentRT" "/Game/Materials/RT_Test_A.RT_Test_A")
  (Utilities|Time|SetTimerbyEvent (delegate Custom|DecayTick) (Variables|Default|GetDecayInterval) true))

(event EventTick
  (params (DeltaSeconds :type Float%20%28single-precision%29))
  (bind _returnvalue (Game|Player|GetPlayerPawn 0))
  (bind _mid (Variables|Default|GetMID))
  (bind _mid_path (Variables|Default|GetMID_Path))
  (bind _mid_2 (Variables|Default|GetMID))
  (bind _mid_3 (Variables|Default|GetMID))
  (bind _returnvalue_2 (Transformation|GetActorLocation _returnvalue))
  (bind _returnvalue_3 (CallFunction|MakeStampPosition _returnvalue_2))
  (if (> (Math|Vector|VectorLength (- _returnvalue_2 (Variables|Default|GetLastStampLocation))) (Variables|Default|GetMinStampDistance))
    (Rendering|Material|SetVectorParameterValue (Variables|Default|GetMID) "StampCenter" _returnvalue_3 :!class /Script/Engine.MaterialInstanceDynamic)
    (Rendering|Material|SetVectorParameterValue (Variables|Default|GetMID) "StampSize" (CallFunction|MakeStampSize) :!class /Script/Engine.MaterialInstanceDynamic)
    (Rendering|Material|SetScalarParameterValue _mid_3 "StampStrength" 0.15 :!class /Script/Engine.MaterialInstanceDynamic)
    (Rendering|Material|SetScalarParameterValue _mid_3 "Decay" 1.0 :!class /Script/Engine.MaterialInstanceDynamic)
    (if (Variables|Default|GetUseA_Decay)
      (Rendering|Material|SetTextureParameterValue _mid_2 "PreviousRT" "/Game/Materials/RT_Test_A.RT_Test_A")
      (Rendering|DrawMaterialtoRenderTarget "/Game/Materials/RT_Test_B.RT_Test_B" _mid)
      (Rendering|Material|SetTextureParameterValue _mid_path "CurrentRT" "/Game/Materials/RT_Test_B.RT_Test_B")
      (else
        (Rendering|Material|SetTextureParameterValue _mid_2 "PreviousRT" "/Game/Materials/RT_Test_B.RT_Test_B")
        (Rendering|DrawMaterialtoRenderTarget "/Game/Materials/RT_Test_A.RT_Test_A" _mid)
        (Rendering|Material|SetTextureParameterValue _mid_path "CurrentRT" "/Game/Materials/RT_Test_A.RT_Test_A")))
    (Variables|Default|SetLastStampLocation (Transformation|GetActorLocation (Game|Player|GetPlayerPawn 0)))
    (Variables|Default|SetUseA_Decay (not (Variables|Default|GetUseA_Decay)))))

(fn ConstructionScript
  (Variables|Default|SetDecay (Math|Float|Power 0.5 (/ (Variables|Default|GetDecayInterval) (Variables|Default|GetDecayHalfLife)))))

(fn ReferencePlanesTransform
  (params (RefPlaneActor :type Actor%20Object%20Reference))
  (bind (_origin _boxextent) (Collision|GetActorBounds RefPlaneActor false false))
  (Variables|Default|SetPlaneTransform (Transformation|GetActorTransform RefPlaneActor))
  (Variables|Default|SetPlaneOrigin _origin)
  (Variables|Default|SetPlaneHalfExtent _boxextent))

(fn ClearAllRTs
  (Rendering|ClearRenderTarget2D "/Game/Materials/RT_Test_A.RT_Test_A")
  (Rendering|ClearRenderTarget2D "/Game/Materials/RT_Test_B.RT_Test_B"))

(fn MakeStampPosition
  (params (PawnLocation :type Vector))
  (bind (_x _y) (Math|Vector|BreakVector PawnLocation))
  (bind _returnvalue (CallFunction|MakeStampSize))
  (bind _planehalfextent (Variables|Default|GetPlaneHalfExtent))
  (bind _planeorigin (Variables|Default|GetPlaneOrigin))
  (bind (_r _g) (Utilities|Struct|BreakLinearColor _returnvalue))
  (return (Math|Conversions|ToLinearColor(Vector) (Math|Vector|MakeVector (+ (/ (+ (- _x (.x _planeorigin)) (.x _planehalfextent)) (* (.x _planehalfextent) 2.0)) (* _r 0.5)) (+ (/ (+ (- _y (.y _planeorigin)) (.y _planehalfextent)) (* (.y _planehalfextent) 2.0)) (* _g 0.5)) 0.0))))

(fn MakeStampSize
  (return (Math|Conversions|ToLinearColor(Vector) (Math|Vector|MakeVector (/ (Variables|Default|GetFootprintWorldSize) (* (.x (Variables|Default|GetPlaneHalfExtent)) 2.0)) (/ (Variables|Default|GetFootprintWorldSize) (* (.y (Variables|Default|GetPlaneHalfExtent)) 2.0)) 0.0))))